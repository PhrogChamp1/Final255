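; Wine bottle clue pickup that the player collects by holding interact, marking its entry in the character's clue array.
; Box overlap with the player's InteractCollider sets the in-range and interaction flags, and Tick polls the character's HoldTime against a threshold.
; Collection plays a journal sound, shows a ClueNotif widget, hides the bottle, then removes both after a delay.
; On BeginPlay it destroys itself if the clue is already found.
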(event OnComponentBeginOverlap(Box)
  (params (OverlappedComponent :type Primitive%20Component%20Object%20Reference) (OtherActor :type Actor%20Object%20Reference) (OtherComp :type Primitive%20Component%20Object%20Reference) (OtherBodyIndex :type Integer) (bFromSweep :type Boolean) (SweepResult :type Hit%20Result%20Structure%20%28by%20ref%29))
  ;[1 1 1] Begin Interact Overlap
  (bind _asbp_first_person_character (Utilities|Casting|CastToBP_FirstPersonCharacter (Game|GetPlayerCharacter 0)))
  (if (== OtherComp (Variables|/Game/FirstPerson/Blueprints/BP_FirstPersonCharacter.BP_FirstPersonCharacter_C|GetInteract%20collider _asbp_first_person_character))
    (Variables|/Game/FirstPerson/Blueprints/BP_FirstPersonCharacter.BP_FirstPersonCharacter_C|SetE_Held _asbp_first_person_character false)
    (Variables|Default|Setinrange true)
    (Development|PrintString "Hello")
    (Variables|/Game/FirstPerson/Blueprints/BP_FirstPersonCharacter.BP_FirstPersonCharacter_C|SetInteractCollision _asbp_first_person_character true)))

(event OnComponentEndOverlap(Box)
  (params (OverlappedComponent :type Primitive%20Component%20Object%20Reference) (OtherActor :type Actor%20Object%20Reference) (OtherComp :type Primitive%20Component%20Object%20Reference) (OtherBodyIndex :type Integer))
  ;[1 1 1] End Interact Overlap
  (bind _asbp_first_person_character (Utilities|Casting|CastToBP_FirstPersonCharacter (Game|GetPlayerCharacter 0)))
  (if (== OtherComp (Variables|/Game/FirstPerson/Blueprints/BP_FirstPersonCharacter.BP_FirstPersonCharacter_C|GetInteract%20collider _asbp_first_person_character))
    (Variables|/Game/FirstPerson/Blueprints/BP_FirstPersonCharacter.BP_FirstPersonCharacter_C|SetE_Held _asbp_first_person_character false)
    (Variables|Default|Setinrange false)
    (Development|PrintString "CollisionEnd")
    (Variables|/Game/FirstPerson/Blueprints/BP_FirstPersonCharacter.BP_FirstPersonCharacter_C|SetInteractCollision _asbp_first_person_character false)))

(event EventBeginPlay
  (Utilities|FlowControl|DelayUntilNextTick)
  (bind _asbp_first_person_character (Utilities|Casting|CastToBP_FirstPersonCharacter (Game|GetPlayerCharacter 0)))
  (if (Utilities|Array|Get(acopy) (Variables|/Game/FirstPerson/Blueprints/BP_FirstPersonCharacter.BP_FirstPersonCharacter_C|GetCluesVar _asbp_first_person_character) 1)
    (Actor|DestroyActor)))

(event Collision|EventActorBeginOverlap
  (params (OtherActor :type Actor%20Object%20Reference)))

(event EventTick
  (params (DeltaSeconds :type Float%20%28single-precision%29))
  ;[1 1 1] On Tick Check for overlap and hold time
  (if (Variables|Default|Getinrange)
    (if (>= (Variables|/Game/FirstPerson/Blueprints/BP_FirstPersonCharacter.BP_FirstPersonCharacter_C|GetHold%20time (stale OnComponentBeginOverlap(Box) _asbp_first_person_character)) 1.5)
      (Utilities|Array|SetArrayElem (Variables|/Game/FirstPerson/Blueprints/BP_FirstPersonCharacter.BP_FirstPersonCharacter_C|GetCluesVar (stale OnComponentBeginOverlap(Box) _asbp_first_person_character)) 1 true)
      (Audio|PlaySound2D "/Game/Sounds/Journal_Entry_-_Made_with_Clipchamp.Journal_Entry_-_Made_with_Clipchamp" 1.0 1.0 0.0 0 0)
      (bind _returnvalue (UserInterface|CreateWidget "/Game/UI_Widgets/ClueNotif.ClueNotif_C" (Game|GetPlayerController 0)))
      (UserInterface|Viewport|AddtoViewport _returnvalue 0)
      (Collision|SetCollisionEnabled (Variables|Default|GetBox) "NoCollision")
      (Rendering|SetActorHiddenInGame true)
      (Utilities|FlowControl|Delay 3.0)
      (Widget|RemovefromParent _returnvalue)
      (Actor|DestroyActor))))

(fn ConstructionScript)