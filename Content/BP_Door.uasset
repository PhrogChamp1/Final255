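; BP_Door is an interactable that opens a Map widget when the player holds interact in range.
; Box overlaps with the first-person character's InteractCollider set the range flag and the character's interaction state.
; Tick watches the character's HoldTime for a narrow window around 1.5 seconds, then pauses the game and shows the map with UI-only input.
; A Mapcreate flag prevents duplicate widgets until the overlap ends.
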(event OnComponentBeginOverlap(Box)
  (params (OverlappedComponent :type Primitive%20Component%20Object%20Reference) (OtherActor :type Actor%20Object%20Reference) (OtherComp :type Primitive%20Component%20Object%20Reference) (OtherBodyIndex :type Integer) (bFromSweep :type Boolean) (SweepResult :type Hit%20Result%20Structure%20%28by%20ref%29))
  ;[1 1 1] Begin Interact Overlap
  (bind _asbp_first_person_character (Utilities|Casting|CastToBP_FirstPersonCharacter (Game|GetPlayerCharacter 0)))
  (if (== OtherComp (Variables|/Game/FirstPerson/Blueprints/BP_FirstPersonCharacter.BP_FirstPersonCharacter_C|GetInteract%20collider _asbp_first_person_character))
    (Variables|/Game/FirstPerson/Blueprints/BP_FirstPersonCharacter.BP_FirstPersonCharacter_C|SetE_Held _asbp_first_person_character false)
    (Variables|Default|Setinrange true)
    (Development|PrintString "Hello")
    (Variables|/Game/FirstPerson/Blueprints/BP_FirstPersonCharacter.BP_FirstPersonCharacter_C|SetInteractCollision _asbp_first_person_character true)))

(event OnComponentEndOverlap(Box)
  (params (OverlappedComponent :type Primitive%20Component%20Object%20Reference) (OtherActor :type Actor%20Object%20Reference) (OtherComp :type Primitive%20Component%20Object%20Reference) (OtherBodyIndex :type Integer))
  ;[1 1 1] End Interact Overlap
  (bind _asbp_first_person_character (Utilities|Casting|CastToBP_FirstPersonCharacter (Game|GetPlayerCharacter 0)))
  (if (== OtherComp (Variables|/Game/FirstPerson/Blueprints/BP_FirstPersonCharacter.BP_FirstPersonCharacter_C|GetInteract%20collider _asbp_first_person_character))
    (Variables|/Game/FirstPerson/Blueprints/BP_FirstPersonCharacter.BP_FirstPersonCharacter_C|SetE_Held _asbp_first_person_character false)
    (Variables|Default|Setinrange false)
    (Development|PrintString "CollisionEnd")
    (Variables|/Game/FirstPerson/Blueprints/BP_FirstPersonCharacter.BP_FirstPersonCharacter_C|SetInteractCollision _asbp_first_person_character false)
    (Variables|Default|Setmapcreate false)))

(event EventBeginPlay)

(event Collision|EventActorBeginOverlap
  (params (OtherActor :type Actor%20Object%20Reference)))

(event EventTick
  (params (DeltaSeconds :type Float%20%28single-precision%29))
  (bind _returnvalue (Game|GetPlayerController 0))
  ;[1 1 1] On Tick Check for overlap and hold time
  (if (Variables|Default|Getinrange)
    (if (and (>= (Variables|/Game/FirstPerson/Blueprints/BP_FirstPersonCharacter.BP_FirstPersonCharacter_C|GetHold%20time (stale OnComponentBeginOverlap(Box) _asbp_first_person_character)) 1.5) (<= (Variables|/Game/FirstPerson/Blueprints/BP_FirstPersonCharacter.BP_FirstPersonCharacter_C|GetHold%20time (stale OnComponentBeginOverlap(Box) _asbp_first_person_character)) 1.6))
      (if (not (Variables|Default|Getmapcreate))
        (Game|SetGamePaused true)
        (Variables|/Script/Engine.PlayerController|SetbShowMouseCursor _returnvalue true)
        (bind _returnvalue_2 (UserInterface|CreateWidget "/Game/UI_Widgets/Map.Map_C" _returnvalue))
        (Input|SetInputModeUIOnly _returnvalue _returnvalue_2 "DoNotLock")
        (UserInterface|Viewport|AddtoViewport _returnvalue_2 0)
        (Variables|/Game/FirstPerson/Blueprints/BP_FirstPersonCharacter.BP_FirstPersonCharacter_C|SetIn_menu (stale OnComponentBeginOverlap(Box) _asbp_first_person_character) true)
        (Variables|Default|Setmapcreate true)))))

(fn ConstructionScript)